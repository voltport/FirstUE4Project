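; Mutant Druid mob Blueprint that shows a floating health bar with the mob's name.
; BeginPlay caches the HP_Bar_Widget from the HPBar widget component.
; Each Tick pushes HP normalized against MaxHP and MobName into that widget, polling rather than reacting to changes.
; Tick also billboards the bar by rotating it toward the player character's CameraTP using a look-at rotation.
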(event `self.ReceiveBeginPlay`
  (set `self.Ref HP Bar Widget` (cast `/Game/Mob_and_Enemy/Mutant_Druid/HP_Bar_Widget` (`WidgetComponent.GetUserWidgetObject` (`self.HP_Bar`)) :!pure true)))

(event `self.ReceiveTick`
  (params (DeltaSeconds :type "Float (single-precision)"))
  (bind _hp_bar (`self.HP_Bar`))
  (bind _ref_hp_bar_widget (`self.Ref HP Bar Widget`))
  (`|ExecutionSequence`
    (:`then_0`
      (`ProgressBar.SetPercent` (`/Game/Mob_and_Enemy/Mutant_Druid/HP_Bar_Widget.HP_Bar` _ref_hp_bar_widget) (`KismetMathLibrary.NormalizeToRange` (`self.HP`) 0.0 (`self.Max_HP`)))
      (`TextBlock.SetText` (`/Game/Mob_and_Enemy/Mutant_Druid/HP_Bar_Widget.Mob_Name` _ref_hp_bar_widget) (`self.Mob_Name`)))
    (:`then_1`
      ;[1 1 1] Сравнивает координаты и задает направление одного на другого
      (`SceneComponent.K2_SetWorldRotation` _hp_bar (`KismetMathLibrary.FindLookAtRotation` (`SceneComponent.K2_GetComponentLocation` _hp_bar) (`SceneComponent.K2_GetComponentLocation` (`/Game/Mannequin/Archer/Blueprint/BP_Charapter.CameraTP` (cast `/Game/Mannequin/Archer/Blueprint/BP_Charapter` (`GameplayStatics.GetPlayerCharacter` 0) :!pure true)))) false false))))

(fn `UserConstructionScript`)